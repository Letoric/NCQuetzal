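; Character Blueprint for the NCQuetzal variant of the Quetzal, with server-configurable carry, saddle platform and flight stats.
; Shortly after BeginPlay, the authority reads the NCQuetzal ini section through ShooterGameMode to set grab weight limit, max saddle structures, tamed running speed modifier and max fly speed.
; Any option that is not positive falls back to a hardcoded default.
; The construction script only calls the parent.
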(event `self.ReceiveBeginPlay`
  (bind _charactermovement (`self.CharacterMovement`))
  (`KismetSystemLibrary.Delay` 0.2)
  (`/Engine/EditorBlueprintResources/ActorMacros.Switch Has Authority`
    (:`Authority`
      (bind _asshootergamemode (cast `ShooterGameMode` (`GameplayStatics.GetGameMode`)))
      (`|ExecutionSequence`
        (:`then_0`
          (bind _returnvalue (`ShooterGameMode.GetFloatOptionIni` _asshootergamemode "NCQuetzal" "GrabWeightMax"))
          (if (> _returnvalue 0.0)
            (set `self.GrabWeightThreshold` _returnvalue)
            (else
              (set `self.GrabWeightThreshold` 400.0))))
        (:`then_1`
          (bind _returnvalue_2 (`ShooterGameMode.GetIntOptionIni` _asshootergamemode "NCQuetzal" "MaxPlatformStructures"))
          (if (> _returnvalue_2 0)
            (set `self.MaxSaddleStructuresNum` _returnvalue_2)
            (else
              (set `self.MaxSaddleStructuresNum` 32))))
        (:`then_2`
          (bind _returnvalue_3 (`ShooterGameMode.GetFloatOptionIni` _asshootergamemode "NCQuetzal" "TamedRunningSpeedMulti"))
          (if (> _returnvalue_3 0.0)
            (set `self.TamedRunningSpeedModifier` _returnvalue_3)
            (else
              (set `self.TamedRunningSpeedModifier` 1.0))))
        (:`then_3`
          (bind _returnvalue_4 (`ShooterGameMode.GetFloatOptionIni` _asshootergamemode "NCQuetzal" "MaxFlySpeed"))
          (if (> _returnvalue_4 0.0)
            (set `CharacterMovementComponent.MaxFlySpeed` _returnvalue_4 _charactermovement)
            (else
              (set `CharacterMovementComponent.MaxFlySpeed` 600.0 _charactermovement))))))))

(fn `UserConstructionScript`
  (`parent.UserConstructionScript`))